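; Base block for the Mario platformer that reacts to player hits and can be swapped out during a P-Block effect.
; It caches the player controller and calls HitBlock when the player character strikes the cube with a straight vertical impact normal.
; PBlockOn hides the cube, disables its collision and spawns a configured substitute actor in its place.
; PBlockOff restores the cube and removes the substitute, or destroys the block if the substitute is no longer valid.
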(event OnComponentHit(Cube)
  (params (HitComponent :type Primitive%20Component%20Object%20Reference) (OtherActor :type Actor%20Object%20Reference) (OtherComp :type Primitive%20Component%20Object%20Reference) (NormalImpulse :type Vector :default "0, 0, 0") (Hit :type Hit%20Result%20Structure%20%28by%20ref%29))
  ;[1 1 1] Get Hit
  (if (and (== OtherActor (Game|GetPlayerCharacter 0)) (== (.Z (Math|Vector|BreakVector (.ImpactNormal (Collision|BreakHitResult Hit)))) 1.0))
    (CallFunction|HitBlock)))

(event EventBeginPlay
  ;[1 1 1] Get Player Controller
  (bind _asbp_player_controller (Utilities|Casting|CastToBP_PlayerController (Game|GetPlayerController 0)))
  (Variables|Default|SetPlayerController _asbp_player_controller))

(fn ConstructionScript)

(fn PBlockon
  (bind _cube (Variables|Default|GetCube))
  (if (not (Variables|Spawn|GetOnPBlock))
    (Rendering|SetVisibility _cube false false)
    (Collision|SetCollisionEnabled _cube "NoCollision")
    (bind _returnvalue (Game|SpawnActorfromClass (Variables|Spawn|GetSpawnActorClass) (Transformation|GetActorTransform) "Undefined" "MultiplyWithRoot" 0 0))
    (Variables|Spawn|SetSpawnActor _returnvalue)
    (Variables|Spawn|SetOnPBlock true)))

(fn PBlockOff
  (bind _cube (Variables|Default|GetCube))
  (bind _spawnactor (Variables|Spawn|GetSpawnActor))
  (Rendering|SetVisibility _cube true false)
  (Collision|SetCollisionEnabled _cube "QueryAndPhysics")
  (Utilities|IsValid _spawnactor
    (:Is%20Valid
      (Actor|DestroyActor _spawnactor)
      (Variables|Spawn|SetOnPBlock false))
    (:Is%20Not%20Valid
      (Actor|DestroyActor))))