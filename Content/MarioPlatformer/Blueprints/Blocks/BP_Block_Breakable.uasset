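; BP_Block_Breakable is a breakable brick block for a Mario-style platformer, built on a parent Blueprint.
; When hit, it checks whether player 0's character has the Fire Flower.
; If so, it plays interaction sound and effects, spawns a points actor, adds the score to the player controller and destroys itself.
; Otherwise it plays a bump sound while a timeline moves its cube mesh vertically.
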(event EventBeginPlay
  (|CallParentFunction))

(event EventHitBlock
  (bind _points (Variables|Default|GetPoints))
  (bind _asbp_third_person_character (Utilities|Casting|CastToBP_ThirdPersonCharacter (Game|GetPlayerCharacter 0)))
  (if (Variables|/Game/ThirdPerson/Blueprints/BP_ThirdPersonCharacter.BP_ThirdPersonCharacter_C|GetHasFireFlower _asbp_third_person_character)
    (Utilities|FlowControl|Sequence
      (:then_0
        (CallFunction|PlayBlockInteractFX (Variables|Default|GetInteractSFX) (Variables|Default|GetInteractVFS%28Niagara%29) (Variables|Default|GetInteractVFS%28Particle%29) (Transformation|GetActorLocation)))
      (:then_1
        (Game|SpawnActorfromClass "/Game/MarioPlatformer/Blueprints/BP_Points.BP_Points_C" (Transformation|GetActorTransform) "Undefined" "MultiplyWithRoot" 0 _points 0)
        (Default|AddPoints (Variables|Default|GetPlayerController) _points))
      (:then_2
        (Actor|DestroyActor)))
    (else
      ;[1 1 1] Move Up and Down
      (Audio|PlaySound2D "/Game/MarioPlatformer/Audio/Mario_BrickBump.Mario_BrickBump" 1.0 1.0 0.0 0 0)
      (bind _movement (Timeline|Timeline PlayFromStart)
        (:Update
          (Transformation|SetRelativeLocation (Variables|Default|GetCube) (Math|Vector|MakeVector 0.0 0.0 _movement) false false))))))

(fn ConstructionScript
  (|CallParentFunction))