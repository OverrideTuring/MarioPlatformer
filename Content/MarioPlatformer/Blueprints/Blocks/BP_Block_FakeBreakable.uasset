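; BP_Block_FakeBreakable is a Mario-style platformer block that, going by its name, poses as breakable but pays out a one-time reward instead of breaking.
; The first hit plays interact effects, swaps the cube's material, spawns points and coin actors while crediting the player controller, and bumps the cube vertically through a timeline.
; An Interacted flag makes later hits play only a brick bump sound.
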(event EventBeginPlay
  (|CallParentFunction))

(event EventHitBlock
  (bind _points (Variables|Default|GetPoints))
  (if (Variables|Default|GetInteracted)
    (Audio|PlaySound2D "/Game/MarioPlatformer/Audio/Mario_BrickBump.Mario_BrickBump" 1.0 1.0 0.0 0 0)
    (else
      (Variables|Default|SetInteracted true)
      (Utilities|FlowControl|Sequence
        (:then_0
          ;[1 1 1] Play Sound and Set Material
          (CallFunction|PlayBlockInteractFX (Variables|Default|GetInteractSFX) (Variables|Default|GetInteractVFS%28Niagara%29) (Variables|Default|GetInteractVFS%28Particle%29) (+ (Transformation|GetActorLocation) "0.000000,0.000000,50.000000"))
          (Rendering|Material|SetMaterial (Variables|Default|GetCube) 0 (Variables|Default|GetInteractMaterial)))
        (:then_1
          ;[1 1 1] Add Points
          (Game|SpawnActorfromClass "/Game/MarioPlatformer/Blueprints/BP_Points.BP_Points_C" (Transformation|GetActorTransform) "Undefined" "MultiplyWithRoot" 0 _points 0)
          (Default|AddPoints (Variables|Default|GetPlayerController) _points))
        (:then_2
          ;[1 1 1] Add Coins
          (Game|SpawnActorfromClass "/Game/MarioPlatformer/Blueprints/Blocks/BP_BlockCoin.BP_BlockCoin_C" (Transformation|GetActorTransform) "Undefined" "MultiplyWithRoot" 0 0)
          (Default|AddCoins (Variables|Default|GetPlayerController) (Variables|Default|GetNumCoins)))
        (:then_3
          ;[1 1 1] Move Up and Down
          (bind _movement (Timeline|Block%20Animation PlayFromStart)
            (:Update
              (Transformation|SetRelativeLocation (Variables|Default|GetCube) (Math|Vector|MakeVector 0.0 0.0 _movement) false false))))))))

(fn ConstructionScript
  (|CallParentFunction))