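; Mario-style item block that, on its first hit, releases a Fire Flower pickup; later hits only play a bump sound.
; HitBlock plays interact FX, swaps the cube material and runs timelines that bounce the block and raise the flower.
; When the flower finishes rising, a pickup Niagara effect spawns and its collision box turns on.
; Character overlap grants the Fire Flower, spawns and awards points, then removes the flower components, leaving the block.
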(event OnComponentBeginOverlap(FlowerBox)
  (params (OverlappedComponent :type Primitive%20Component%20Object%20Reference) (OtherActor :type Actor%20Object%20Reference) (OtherComp :type Primitive%20Component%20Object%20Reference) (OtherBodyIndex :type Integer) (bFromSweep :type Boolean) (SweepResult :type Hit%20Result%20Structure%20%28by%20ref%29))
  (bind _points (Variables|Default|GetPoints))
  (bind _asbp_third_person_character (Utilities|Casting|CastToBP_ThirdPersonCharacter OtherActor))
  (Default|GetFireFlower _asbp_third_person_character)
  (Utilities|FlowControl|Sequence
    (:then_0
      ;[1 1 1] Add Points
      (Game|SpawnActorfromClass "/Game/MarioPlatformer/Blueprints/BP_Points.BP_Points_C" (Transformation|GetWorldTransform (Variables|Default|GetArrow)) "Undefined" "MultiplyWithRoot" 0 _points 0)
      (Default|AddPoints (Variables|Default|GetPlayerController) _points))
    (:then_1
      ;[1 1 1] Destroy Components
      (Components|Activation|Deactivate (Variables|Default|GetFlowerVFX))
      (Components|DestroyComponent (Variables|Default|GetFlower)))))

(event EventBeginPlay
  (|CallParentFunction))

(event EventHitBlock
  (if (Variables|Default|GetInteracted)
    (Audio|PlaySound2D "/Game/MarioPlatformer/Audio/Mario_BrickBump.Mario_BrickBump" 1.0 1.0 0.0 0 0)
    (else
      (Variables|Default|SetInteracted true)
      (Utilities|FlowControl|Sequence
        (:then_0
          ;[1 1 1] Play Sound and Set Material
          (CallFunction|PlayBlockInteractFX (Variables|Default|GetInteractSFX) (Variables|Default|GetInteractVFS%28Niagara%29) (Variables|Default|GetInteractVFS%28Particle%29) (+ (Transformation|GetActorLocation) "0.000000,0.000000,50.000000"))
          (Rendering|Material|SetMaterial (Variables|Default|GetCube) 0 (Variables|Default|GetInteractMaterial)))
        (:then_1
          ;[1 1 1] Move Up and Down
          (bind _movement (Timeline|Block%20Animation PlayFromStart)
            (:Update
              (Transformation|SetRelativeLocation (Variables|Default|GetCube) (Math|Vector|MakeVector 0.0 0.0 _movement) false false))))
        (:then_2
          ;[1 1 1] Move Flower Up
          (bind _movement_2 (Timeline|Flower%20Animation PlayFromStart)
            (:Update
              (Transformation|SetRelativeLocation (Variables|Default|GetFlower) (Math|Vector|MakeVector 0.0 0.0 _movement_2) false false))
            (:Finished
              (bind _returnvalue (Niagara|SpawnSystematLocation "/Game/Stylized_VFX_StPack/Particles/P_PickUp.P_PickUp" (+ (Transformation|GetWorldLocation (Variables|Default|GetFlower)) "0.000000,0.000000,-50.000000")))
              (Variables|Default|SetFlowerVFX _returnvalue)
              (Collision|SetCollisionEnabled (Variables|Default|GetFlowerBox) "QueryOnly"))))))))

(fn ConstructionScript
  (|CallParentFunction))