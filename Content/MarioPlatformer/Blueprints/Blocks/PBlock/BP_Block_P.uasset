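; P-switch block that the player smashes by landing on it, switching tagged BP_Block_Base actors on for a timed duration.
; The hit plays effects, shakes camera and controller, swaps to the smashed mesh and pauses level music for P-block audio.
; A shared BP_SingletonManager, spawned if missing, holds that audio and the timer, so each press restarts the countdown.
; Timeout, player death or level completion switches the blocks off and restores the music.
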(event OnComponentHit(BoxCollision)
  (params (HitComponent :type Primitive%20Component%20Object%20Reference) (OtherActor :type Actor%20Object%20Reference) (OtherComp :type Primitive%20Component%20Object%20Reference) (NormalImpulse :type Vector :default "0, 0, 0") (Hit :type Hit%20Result%20Structure%20%28by%20ref%29))
  (bind _block_p (Variables|Default|GetBlock_P))
  (bind _singletonmanager (Variables|Default|GetSingletonManager))
  (bind _returnvalue (Transformation|GetWorldTransform _block_p))
  (bind _audio (Variables|/Game/MarioPlatformer/Blueprints/Blocks/PBlock/BP_SingletonManager.BP_SingletonManager_C|GetAudio _singletonmanager))
  (bind _asbp_third_person_character (Utilities|Casting|CastToBP_ThirdPersonCharacter OtherActor))
  (if (Utilities|Operators|EqualEqual (.ImpactNormal (Collision|BreakHitResult Hit)) "0.000000,0.000000,-1.000000" 0.01)
    (EventDispatchers|AssignPlayerDeathSequence _asbp_third_person_character (delegate Custom|Player%20Death%20Sequence_Event))
    (Utilities|FlowControl|Sequence
      (:then_0
        ;[1 1 1] Play Sound and VFX
        (Audio|PlaySound2D "/Game/MarioPlatformer/Audio/Mario_Thwomp.Mario_Thwomp" 1.0 1.0 0.0 0 0)
        (Niagara|SpawnSystematLocation "/Game/Stylized_VFX_StPack/Particles/P_Hits.P_Hits" (.location _returnvalue) (.rotation _returnvalue) (.scale _returnvalue))
        (if (not (Audio|Components|Audio|IsPlaying _audio))
          (Audio|Components|Audio|Play _audio 0.0)
          (Class|AudioComponent|SetPaused (Variables|/Game/MarioPlatformer/Blueprints/BP_LevelSettings.BP_LevelSettings_C|GetLevelMusic (Variables|Default|GetLevelSettings)) true)))
      (:then_1
        ;[1 1 1] Camera and Controller Shake
        (Camera|PlayWorldCameraShake "/Game/MarioPlatformer/Blueprints/Blocks/PBlock/BP_CamaraShake.BP_CamaraShake_C" (Transformation|GetWorldLocation (Variables|Default|GetBlock_P)) 1e+03 2e+03)
        (Game|Feedback|ClientPlayForceFeedback (Game|GetPlayerController 0) "/Game/MarioPlatformer/Blueprints/Blocks/PBlock/ForceFeedback.ForceFeedback" "None" false false false))
      (:then_2
        ;[1 1 1] Set Visibility and Destroy Components
        (Rendering|SetVisibility (Variables|Default|GetBlock_P_Top_Smashed) true false)
        (Components|DestroyComponent (Variables|Default|GetBoxCollision)))
      (:then_3
        ;[1 1 1] PBlock On
        (bind _outactors (Actor|GetAllActorsOfClasswithTag "/Game/MarioPlatformer/Blueprints/Blocks/BP_Block_Base.BP_Block_Base_C" (Variables|Default|GetTag)))
        (bind _output_get (Variables|Default|SetBlocks _outactors))
        (for _array_element _output_get
          (Default|PBlockon _array_element))
        (Utilities|Time|ClearandInvalidateTimerbyHandle (Variables|/Game/MarioPlatformer/Blueprints/Blocks/PBlock/BP_SingletonManager.BP_SingletonManager_C|GetTimerHandler (Variables|Default|GetSingletonManager))))
      (:then_4
        ;[1 1 1] PBlock Off
        (bind _returnvalue_2 (Utilities|Time|SetTimerbyEvent (delegate Custom|PBlock%20Time%20Over) (Variables|Default|GetDuration)))
        (Variables|/Game/MarioPlatformer/Blueprints/Blocks/PBlock/BP_SingletonManager.BP_SingletonManager_C|SetTimerHandler (Variables|Default|GetSingletonManager) _returnvalue_2)))))

(event Custom|PBlock%20Time%20Over
  ;[1 1 1] PBlock Off
  (for _array_element (Variables|Default|GetBlocks)
    (Utilities|IsValid _array_element
      (:Is%20Valid
        (Default|PBlockOff _array_element))))
  (Audio|Components|Audio|FadeOut (Variables|/Game/MarioPlatformer/Blueprints/Blocks/PBlock/BP_SingletonManager.BP_SingletonManager_C|GetAudio (Variables|Default|GetSingletonManager)) 1.0 0.0 "Linear" :!class /Script/Engine.AudioComponent)
  (Class|AudioComponent|SetPaused (Variables|/Game/MarioPlatformer/Blueprints/BP_LevelSettings.BP_LevelSettings_C|GetLevelMusic (Variables|Default|GetLevelSettings)) false))

(event Custom|Player%20Death%20Sequence_Event
  (Utilities|Time|ClearandInvalidateTimerbyHandle (Variables|/Game/MarioPlatformer/Blueprints/Blocks/PBlock/BP_SingletonManager.BP_SingletonManager_C|GetTimerHandler (Variables|Default|GetSingletonManager)))
  ;[1 1 1] PBlock Off
  (for _array_element (Variables|Default|GetBlocks)
    (Utilities|IsValid _array_element
      (:Is%20Valid
        (Default|PBlockOff _array_element))))
  (Audio|Components|Audio|FadeOut (Variables|/Game/MarioPlatformer/Blueprints/Blocks/PBlock/BP_SingletonManager.BP_SingletonManager_C|GetAudio (Variables|Default|GetSingletonManager)) 1.0 0.0 "Linear" :!class /Script/Engine.AudioComponent)
  (Class|AudioComponent|SetPaused (Variables|/Game/MarioPlatformer/Blueprints/BP_LevelSettings.BP_LevelSettings_C|GetLevelMusic (Variables|Default|GetLevelSettings)) false))

(event Custom|Level%20Complete_Event
  ;[1 1 1] Set P Block Off at the End of the Level
  (Utilities|Time|ClearandInvalidateTimerbyHandle (Variables|/Game/MarioPlatformer/Blueprints/Blocks/PBlock/BP_SingletonManager.BP_SingletonManager_C|GetTimerHandler (Variables|Default|GetSingletonManager)))
  (CallFunction|PBlockTimeOver))

(event EventBeginPlay
  ;[1 1 1] Get Singleton Manager
  (bind _returnvalue (Actor|GetActorOfClass "/Game/MarioPlatformer/Blueprints/Blocks/PBlock/BP_SingletonManager.BP_SingletonManager_C"))
  (if (== _returnvalue 0)
    (bind _returnvalue_2 (Game|SpawnActorfromClass "/Game/MarioPlatformer/Blueprints/Blocks/PBlock/BP_SingletonManager.BP_SingletonManager_C" (Transformation|GetActorTransform) "Undefined" "MultiplyWithRoot" 0 0))
    (Variables|Default|SetSingletonManager _returnvalue_2)
    ;[1 1 1] Set P Block Off at the End of the Level
    (EventDispatchers|AssignLevelComplete (Variables|Default|GetEndLevelFlag) (delegate Custom|Level%20Complete_Event))
    (else
      (Variables|Default|SetSingletonManager _returnvalue))))

(fn ConstructionScript)