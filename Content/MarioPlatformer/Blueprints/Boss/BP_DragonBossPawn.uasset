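; BP_DragonBossPawn is the dragon boss pawn, which wakes when the player comes near.
; The first time the player character overlaps its SphereCollision, a DoOnce sets the Awaken flag and plays a scream montage on the Dragon mesh after a short delay.
; The same trigger also casts the player to BP_ThirdPersonCharacter and stores it as the Player reference.
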(event OnComponentBeginOverlap(SphereCollision)
  (params (OverlappedComponent :type Primitive%20Component%20Object%20Reference) (OtherActor :type Actor%20Object%20Reference) (OtherComp :type Primitive%20Component%20Object%20Reference) (OtherBodyIndex :type Integer) (bFromSweep :type Boolean) (SweepResult :type Hit%20Result%20Structure%20%28by%20ref%29))
  (bind _returnvalue (Game|GetPlayerCharacter 0))
  ;[1 1 1] Meet Player
  (if (== OtherActor _returnvalue)
    (Utilities|FlowControl|DoOnce false
      (:Completed
        (Utilities|FlowControl|Sequence
          (:then_0
            (Variables|Default|SetAwaken true)
            (Utilities|FlowControl|Delay 2.0)
            (Animation|Montage|PlayMontage (Variables|Default|GetDragon) "/Game/MarioPlatformer/Blueprints/Boss/Montage/AM_ScreamAnim.AM_ScreamAnim"))
          (:then_1
            (bind _asbp_third_person_character (Utilities|Casting|CastToBP_ThirdPersonCharacter _returnvalue))
            (Variables|Default|SetPlayer _asbp_third_person_character)))))))

(fn ConstructionScript)