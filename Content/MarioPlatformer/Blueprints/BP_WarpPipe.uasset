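; Mario-style warp pipe that carries the third-person character to a linked ConnectedPipe.
; An overlap-controlled gate admits down input on down pipes and up input on others, then disables movement and collision.
; Timelines slide the capsule into this pipe and out of the linked exit by each pipe's orientation, with warp sounds, before restoring control.
; The construction script stacks instanced body segments up or down from PipeEnd's Z.
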(event OnComponentBeginOverlap(Collision)
  (params (OverlappedComponent :type Primitive%20Component%20Object%20Reference) (OtherActor :type Actor%20Object%20Reference) (OtherComp :type Primitive%20Component%20Object%20Reference) (OtherBodyIndex :type Integer) (bFromSweep :type Boolean) (SweepResult :type Hit%20Result%20Structure%20%28by%20ref%29))
  (bind _exitstart (Variables|Default|GetExitStart))
  (bind _warpinpoint (Variables|Default|GetWarpInPoint))
  (bind _warpinpoint_2 (Variables|Default|GetWarpInPoint))
  (bind _exitstart_2 (Variables|Default|GetExitStart))
  (bind _returnvalue (Transformation|GetWorldLocation _warpinpoint))
  (bind _returnvalue_2 (Transformation|GetWorldLocation _warpinpoint_2))
  (bind _asbp_third_person_character (Utilities|Casting|CastToBP_ThirdPersonCharacter OtherActor))
  (Utilities|FlowControl|Gate true) ; enters at Open
)

(event OnComponentEndOverlap(Collision)
  (params (OverlappedComponent :type Primitive%20Component%20Object%20Reference) (OtherActor :type Actor%20Object%20Reference) (OtherComp :type Primitive%20Component%20Object%20Reference) (OtherBodyIndex :type Integer))
  (bind _exitstart (Variables|Default|GetExitStart))
  (bind _warpinpoint (Variables|Default|GetWarpInPoint))
  (bind _warpinpoint_2 (Variables|Default|GetWarpInPoint))
  (bind _exitstart_2 (Variables|Default|GetExitStart))
  (bind _returnvalue (Transformation|GetWorldLocation _warpinpoint))
  (bind _returnvalue_2 (Transformation|GetWorldLocation _warpinpoint_2))
  (Utilities|Casting|CastToBP_ThirdPersonCharacter OtherActor)
  (Utilities|FlowControl|Gate true) ; enters at Close
)

(event Input|EnhancedActionEvents|EnhancedInputActionIA_JumpDown
  (params (ActionValue :type Boolean) (ElapsedSeconds :type Float%20%28double-precision%29) (TriggeredSeconds :type Float%20%28double-precision%29) (InputAction :type Input%20Action%20Object%20Reference :default "/Game/ThirdPerson/Input/Actions/IA_JumpDown.IA_JumpDown"))
  (bind _exitstart (Variables|Default|GetExitStart))
  (bind _warpinpoint (Variables|Default|GetWarpInPoint))
  (bind _warpinpoint_2 (Variables|Default|GetWarpInPoint))
  (bind _exitstart_2 (Variables|Default|GetExitStart))
  (bind _returnvalue (Transformation|GetWorldLocation _warpinpoint))
  (bind _returnvalue_2 (Transformation|GetWorldLocation _warpinpoint_2))
  (if (and (Variables|Default|GetCanInteract) (Variables|Default|GetIsDownPipe))
    (Utilities|FlowControl|Gate true
      (:Exit
        (bind _output_get (Variables|Default|SetPlayerCharacter (stale OnComponentBeginOverlap(Collision) _asbp_third_person_character)))
        (Pawn|Components|CharacterMovement|DisableMovement (Variables|/Script/Engine.Character|GetCharacterMovement _output_get))
        (Collision|SetCollisionEnabled (Variables|/Script/Engine.Character|GetCapsuleComponent _output_get) "NoCollision")
        (if (Variables|Default|GetIsDownPipe)
          (Utilities|FlowControl|Sequence
            (:then_0
              ;[1 1 1] Enter Top Down
              (bind _movement (Timeline|Top%20Down%20Timeline PlayFromStart)
                (:Update
                  (Transformation|SetWorldLocation (Variables|/Script/Engine.Character|GetCapsuleComponent (Variables|Default|GetPlayerCharacter)) (Math|Vector|MakeVector (.x _returnvalue) (.y _returnvalue) (+ _movement (.z _returnvalue) (Variables|/Script/Engine.CapsuleComponent|GetCapsuleHalfHeight (Variables|/Script/Engine.Character|GetCapsuleComponent (Variables|Default|GetPlayerCharacter))))) false false))
                (:Finished
                  (Utilities|FlowControl|Delay 0.4 :!label _label)
                  (Audio|PlaySound2D "/Game/MarioPlatformer/Audio/Mario_Warp.Mario_Warp" 1.0 1.0 0.0 0 0)
                  (if (Variables|Default|GetIsExitUp)
                    ;[1 1 1] Exit Bottom Up
                    (bind _movement_2 (Timeline|Bottom%20Up%20Timeline PlayFromStart)
                      (:Update
                        (Transformation|SetWorldLocation (Variables|/Script/Engine.Character|GetCapsuleComponent (Variables|Default|GetPlayerCharacter)) (Math|Vector|MakeVector (.x _exitstart_2) (.y _exitstart_2) (+ _movement_2 (.z _exitstart_2) (Variables|/Script/Engine.CapsuleComponent|GetCapsuleHalfHeight (Variables|/Script/Engine.Character|GetCapsuleComponent (Variables|Default|GetPlayerCharacter))))) false false))
                      (:Finished
                        ;[1 1 1] Enable Player Movement
                        (Pawn|Components|CharacterMovement|SetMovementMode (Variables|/Script/Engine.Character|GetCharacterMovement (Variables|Default|GetPlayerCharacter)) "MOVE_Walking" 0 :!label _label_2)
                        (Collision|SetCollisionEnabled (Variables|/Script/Engine.Character|GetCapsuleComponent (Variables|Default|GetPlayerCharacter)) "QueryAndPhysics")))
                    (else
                      ;[1 1 1] Exit Top Down
                      (bind _movement_3 (Timeline|Reverse%20Top%20Down%20Timeline PlayFromStart)
                        (:Update
                          (Transformation|SetWorldLocation (Variables|/Script/Engine.Character|GetCapsuleComponent (Variables|Default|GetPlayerCharacter)) (Math|Vector|MakeVector (.x _exitstart) (.y _exitstart) (+ _movement_3 (- (.z _exitstart) (Variables|/Script/Engine.CapsuleComponent|GetCapsuleHalfHeight (Variables|/Script/Engine.Character|GetCapsuleComponent (Variables|Default|GetPlayerCharacter)))))) false false))
                        (:Finished
                          (goto _label_2))))))))
            (:then_1
              ;[1 1 1] Play Warp Sound
              (Utilities|FlowControl|Delay 0.2 :!label _label_3)
              (Audio|PlaySound2D "/Game/MarioPlatformer/Audio/Mario_Warp.Mario_Warp" 1.0 1.0 0.0 0 0)))
          (else
            (Utilities|FlowControl|Sequence
              (:then_0
                ;[1 1 1] Enter Bottom Up
                (bind _movement_4 (Timeline|Reverse%20Bottom%20Up%20Timeline PlayFromStart)
                  (:Update
                    (Transformation|SetWorldLocation (Variables|/Script/Engine.Character|GetCapsuleComponent (Variables|Default|GetPlayerCharacter)) (Math|Vector|MakeVector (.x _returnvalue_2) (.y _returnvalue_2) (+ _movement_4 (- (.z _returnvalue_2) (Variables|/Script/Engine.CapsuleComponent|GetCapsuleHalfHeight (Variables|/Script/Engine.Character|GetCapsuleComponent (Variables|Default|GetPlayerCharacter)))))) false false))
                  (:Finished
                    (goto _label))))
              (:then_1
                (goto _label_3)))))))))

(event Input|EnhancedActionEvents|EnhancedInputActionIA_PlayerUp
  (params (ActionValue :type Boolean) (ElapsedSeconds :type Float%20%28double-precision%29) (TriggeredSeconds :type Float%20%28double-precision%29) (InputAction :type Input%20Action%20Object%20Reference :default "/Game/ThirdPerson/Input/Actions/IA_PlayerUp.IA_PlayerUp"))
  (bind _exitstart (Variables|Default|GetExitStart))
  (bind _warpinpoint (Variables|Default|GetWarpInPoint))
  (bind _warpinpoint_2 (Variables|Default|GetWarpInPoint))
  (bind _exitstart_2 (Variables|Default|GetExitStart))
  (bind _returnvalue (Transformation|GetWorldLocation _warpinpoint))
  (bind _returnvalue_2 (Transformation|GetWorldLocation _warpinpoint_2))
  (if (and (not (Variables|Default|GetIsDownPipe)) (Variables|Default|GetCanInteract))
    (Utilities|FlowControl|Gate true
      (:Exit
        (bind _output_get (Variables|Default|SetPlayerCharacter (stale OnComponentBeginOverlap(Collision) _asbp_third_person_character)))
        (Pawn|Components|CharacterMovement|DisableMovement (Variables|/Script/Engine.Character|GetCharacterMovement _output_get))
        (Collision|SetCollisionEnabled (Variables|/Script/Engine.Character|GetCapsuleComponent _output_get) "NoCollision")
        (if (Variables|Default|GetIsDownPipe)
          (Utilities|FlowControl|Sequence
            (:then_0
              ;[1 1 1] Enter Top Down
              (bind _movement (Timeline|Top%20Down%20Timeline PlayFromStart)
                (:Update
                  (Transformation|SetWorldLocation (Variables|/Script/Engine.Character|GetCapsuleComponent (Variables|Default|GetPlayerCharacter)) (Math|Vector|MakeVector (.x _returnvalue) (.y _returnvalue) (+ _movement (.z _returnvalue) (Variables|/Script/Engine.CapsuleComponent|GetCapsuleHalfHeight (Variables|/Script/Engine.Character|GetCapsuleComponent (Variables|Default|GetPlayerCharacter))))) false false))
                (:Finished
                  (Utilities|FlowControl|Delay 0.4 :!label _label)
                  (Audio|PlaySound2D "/Game/MarioPlatformer/Audio/Mario_Warp.Mario_Warp" 1.0 1.0 0.0 0 0)
                  (if (Variables|Default|GetIsExitUp)
                    ;[1 1 1] Exit Bottom Up
                    (bind _movement_2 (Timeline|Bottom%20Up%20Timeline PlayFromStart)
                      (:Update
                        (Transformation|SetWorldLocation (Variables|/Script/Engine.Character|GetCapsuleComponent (Variables|Default|GetPlayerCharacter)) (Math|Vector|MakeVector (.x _exitstart_2) (.y _exitstart_2) (+ _movement_2 (.z _exitstart_2) (Variables|/Script/Engine.CapsuleComponent|GetCapsuleHalfHeight (Variables|/Script/Engine.Character|GetCapsuleComponent (Variables|Default|GetPlayerCharacter))))) false false))
                      (:Finished
                        ;[1 1 1] Enable Player Movement
                        (Pawn|Components|CharacterMovement|SetMovementMode (Variables|/Script/Engine.Character|GetCharacterMovement (Variables|Default|GetPlayerCharacter)) "MOVE_Walking" 0 :!label _label_2)
                        (Collision|SetCollisionEnabled (Variables|/Script/Engine.Character|GetCapsuleComponent (Variables|Default|GetPlayerCharacter)) "QueryAndPhysics")))
                    (else
                      ;[1 1 1] Exit Top Down
                      (bind _movement_3 (Timeline|Reverse%20Top%20Down%20Timeline PlayFromStart)
                        (:Update
                          (Transformation|SetWorldLocation (Variables|/Script/Engine.Character|GetCapsuleComponent (Variables|Default|GetPlayerCharacter)) (Math|Vector|MakeVector (.x _exitstart) (.y _exitstart) (+ _movement_3 (- (.z _exitstart) (Variables|/Script/Engine.CapsuleComponent|GetCapsuleHalfHeight (Variables|/Script/Engine.Character|GetCapsuleComponent (Variables|Default|GetPlayerCharacter)))))) false false))
                        (:Finished
                          (goto _label_2))))))))
            (:then_1
              ;[1 1 1] Play Warp Sound
              (Utilities|FlowControl|Delay 0.2 :!label _label_3)
              (Audio|PlaySound2D "/Game/MarioPlatformer/Audio/Mario_Warp.Mario_Warp" 1.0 1.0 0.0 0 0)))
          (else
            (Utilities|FlowControl|Sequence
              (:then_0
                ;[1 1 1] Enter Bottom Up
                (bind _movement_4 (Timeline|Reverse%20Bottom%20Up%20Timeline PlayFromStart)
                  (:Update
                    (Transformation|SetWorldLocation (Variables|/Script/Engine.Character|GetCapsuleComponent (Variables|Default|GetPlayerCharacter)) (Math|Vector|MakeVector (.x _returnvalue_2) (.y _returnvalue_2) (+ _movement_4 (- (.z _returnvalue_2) (Variables|/Script/Engine.CapsuleComponent|GetCapsuleHalfHeight (Variables|/Script/Engine.Character|GetCapsuleComponent (Variables|Default|GetPlayerCharacter)))))) false false))
                  (:Finished
                    (goto _label))))
              (:then_1
                (goto _label_3)))))))))

(event EventBeginPlay
  (bind _connectedpipe (Variables|Default|GetConnectedPipe)
    (:then
      (Variables|Default|SetExitStart (Transformation|GetWorldLocation (Variables|BP_WarpPipe_C|GetWarpOutPoint _connectedpipe)))
      (Variables|Default|SetIsExitUp (Variables|BP_WarpPipe_C|GetIsDownPipe _connectedpipe)))
    (:else)))

(fn ConstructionScript
  (bind _pipeend (Variables|Default|GetPipeEnd))
  (bind _returnvalue (/ (.z _pipeend) 1e+01))
  (bind _returnvalue_2 (Math|Float|Truncate _returnvalue))
  (if (> _returnvalue_2 0)
    (for _index (range 1 _returnvalue_2)
      (Components|InstancedStaticMesh|AddInstance (Variables|Default|GetPipeBody) (Math|Transform|MakeTransform (Math|Vector|MakeVector 0.0 0.0 (* _index 100)) "0, 0, 0" "1.000000,1.000000,1.000000") false))
    (else
      (for _index_2 (range _returnvalue_2 0)
        (Components|InstancedStaticMesh|AddInstance (Variables|Default|GetPipeBody) (Math|Transform|MakeTransform (Math|Vector|MakeVector 0.0 0.0 (* _index_2 100)) "0, 0, 0" "1.000000,1.000000,1.000000") false)))))