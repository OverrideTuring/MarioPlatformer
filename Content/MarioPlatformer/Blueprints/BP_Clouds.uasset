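; BP_Clouds is an actor that fills a box-shaped area with decorative clouds in the Mario platformer.
; The construction script sizes the SpawnArea box from AreaExtent, then adds NumClouds instances to the Cloud instanced mesh component.
; Each instance gets a random local position within the box, zero rotation and a random uniform scale between MinScale and MaxScale.
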(fn ConstructionScript
  (Components|Box|SetBoxExtent (Variables|Default|GetSpawnArea) (Variables|Default|GetAreaExtent) true)
  (for _index (range 1 (Variables|Default|GetNumClouds))
    (Components|InstancedStaticMesh|AddInstance (Variables|Default|GetCloud) (Math|Transform|MakeTransform (Math|Random|RandomPointinBoundingBox "0, 0, 0" (Components|Box|GetScaledBoxExtent (Variables|Default|GetSpawnArea))) "0, 0, 0" (Math|Conversions|ToVector(Float) (Math|Random|RandomFloatinRange (Variables|Default|GetMinScale) (Variables|Default|GetMaxScale)))) false)))