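; End-of-level flagpole that, on player overlap, disables input, signals level completion once and runs a Mario-style finishing cutscene.
; It snaps flag and player into place by grab height, then uses timed component moves and animations to slide both down and jump the player to an exploding end.
; A looped DoN then spawns point-awarding fireworks at random spots in a box, counted by the formatted time's last digit.
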(event OnComponentBeginOverlap(TriggerVolume)
  (params (OverlappedComponent :type Primitive%20Component%20Object%20Reference) (OtherActor :type Actor%20Object%20Reference) (OtherComp :type Primitive%20Component%20Object%20Reference) (OtherBodyIndex :type Integer) (bFromSweep :type Boolean) (SweepResult :type Hit%20Result%20Structure%20%28by%20ref%29))
  (bind _returnvalue (Game|GetPlayerController 0))
  (bind _flag (Variables|Default|GetFlag))
  (bind _player_end_point (Variables|Default|GetPlayer%20End%20Point))
  (bind _flag_end_point (Variables|Default|GetFlag%20End%20Point))
  (bind _fireworks_area (Variables|Default|GetFireworks%20Area))
  (bind _fireworkspoints (Variables|Default|GetFireworksPoints))
  (bind _flag_2 (Variables|Default|GetFlag))
  (bind _player_explode_point (Variables|Default|GetPlayer%20Explode%20Point))
  (bind _player_start_point (Variables|Default|GetPlayer%20Start%20Point))
  (bind _returnvalue_2 (Transformation|GetWorldLocation _flag))
  (bind _returnvalue_3 (Transformation|GetWorldLocation _player_start_point))
  ;[1 1 1] Collide with Player, Level Completes
  (bind _asbp_third_person_character (Utilities|Casting|CastToBP_ThirdPersonCharacter OtherActor))
  (bind _output_get (Variables|Default|SetPlayerCharacter _asbp_third_person_character))
  (Input|DisableInput _output_get _returnvalue)
  (Utilities|FlowControl|DoOnce false
    (:Completed
      (bind _asbp_player_controller (Utilities|Casting|CastToBP_PlayerController _returnvalue))
      (Variables|Default|SetPlayerController _asbp_player_controller)
      (Default|CallLevelComplete)
      ;[1 1 1] Set Flag to Right Position
      (if (< (.z _returnvalue_2) (.z (Transformation|GetWorldLocation (Variables|/Game/ThirdPerson/Blueprints/BP_ThirdPersonCharacter.BP_ThirdPersonCharacter_C|GetFlagAttachPoint (Variables|Default|GetPlayerCharacter)))))
        (bind _output_get_2 (Variables|Default|SetFlagStartPoint (Math|Vector|MakeVector (.x _returnvalue_2) (.y _returnvalue_2) (.z _returnvalue_2))))
        (Transformation|SetWorldLocation _flag_2 _output_get_2 false false)
        ;[1 1 1] Set Player Location
        (Transformation|SetActorLocation (Variables|Default|GetPlayerCharacter) (Transformation|GetWorldLocation (Variables|Default|GetPlayer%20Start%20Point)) false false)
        (else
          (bind _output_get_3 (Variables|Default|SetFlagStartPoint (Math|Vector|MakeVector (.x _returnvalue_2) (.y _returnvalue_2) (.z (Transformation|GetWorldLocation (Variables|/Game/ThirdPerson/Blueprints/BP_ThirdPersonCharacter.BP_ThirdPersonCharacter_C|GetFlagAttachPoint (Variables|Default|GetPlayerCharacter)))))))
          (Transformation|SetWorldLocation _flag_2 _output_get_3 false false)
          (Transformation|SetActorLocation (Variables|Default|GetPlayerCharacter) (Math|Vector|MakeVector (.x _returnvalue_3) (.y _returnvalue_3) (.z (Transformation|GetActorLocation (Variables|Default|GetPlayerCharacter)))) false false)))
      ;[1 1 1] Set Player Rotation
      (Transformation|SetActorRotation (Variables|Default|GetPlayerCharacter) (Transformation|GetWorldRotation (Variables|Default|GetPlayer%20End%20Point)))
      ;[1 1 1] Stop Movement and Play Animation
      (Components|Activation|Deactivate (Variables|/Script/Engine.Character|GetCharacterMovement (Variables|Default|GetPlayerCharacter)))
      (Components|Animation|PlayAnimation (Variables|/Script/Engine.Character|GetMesh (Variables|Default|GetPlayerCharacter)) "/Game/Characters/Mannequins/Animations/Manny/MM_Run_Fwd.MM_Run_Fwd" false)
      (Components|Animation|SetPosition (Variables|/Script/Engine.Character|GetMesh (Variables|Default|GetPlayerCharacter)) 1.9 true)
      (Utilities|FlowControl|Delay 1.0)
      (Audio|PlaySound2D "/Game/MarioPlatformer/Audio/Mario_FlagPole.Mario_FlagPole" 1.0 1.0 0.0 0 0)
      (Utilities|FlowControl|Sequence
        (:then_0
          ;[1 1 1] Move Player Character Down
          (Components|MoveComponentTo (Variables|/Script/Engine.Character|GetCapsuleComponent (Variables|Default|GetPlayerCharacter)) (Transformation|GetWorldLocation _player_end_point) (Transformation|GetWorldRotation _player_end_point) false false 1.0 false))
        (:then_1
          ;[1 1 1] Move Flag Down
          (Components|MoveComponentTo (Variables|Default|GetFlag) (Variables|/Script/Engine.SceneComponent|GetRelativeLocation _flag_end_point) (Variables|/Script/Engine.SceneComponent|GetRelativeRotation _flag_end_point) false false 1.0 false)
          ;[1 1 1] Jump to Explode Point
          (Components|Animation|PlayAnimation (Variables|/Script/Engine.Character|GetMesh (Variables|Default|GetPlayerCharacter)) "/Game/Characters/Mannequins/Animations/Manny/MM_Jump.MM_Jump" false)
          (Utilities|FlowControl|Delay 0.3)
          (Components|Animation|PlayAnimation (Variables|/Script/Engine.Character|GetMesh (Variables|Default|GetPlayerCharacter)) "/Game/Characters/Mannequins/Animations/Manny/MM_Fall_Loop.MM_Fall_Loop" false)
          (Components|MoveComponentTo (Variables|/Script/Engine.Character|GetCapsuleComponent (Variables|Default|GetPlayerCharacter)) (Transformation|GetWorldLocation _player_explode_point) (Transformation|GetWorldRotation _player_explode_point) false false 0.5 false)
          ;[1 1 1] Explode the Player
          (Audio|PlaySoundatLocation "/Game/StarterContent/Audio/Explosion_Cue.Explosion_Cue" (Transformation|GetWorldLocation (Variables|/Script/Engine.Character|GetCapsuleComponent (Variables|Default|GetPlayerCharacter))) "0, 0, 0" 1.0 1.0 0.0 0 0 0 0)
          (Effects|SpawnEmitteratLocation "/Game/StarterContent/Particles/P_Explosion.P_Explosion" (Transformation|GetWorldLocation (Variables|/Script/Engine.Character|GetCapsuleComponent (Variables|Default|GetPlayerCharacter))) "0, 0, 0" "3.000000,3.000000,3.000000")
          (Rendering|SetVisibility (Variables|/Script/Engine.Character|GetCapsuleComponent (Variables|Default|GetPlayerCharacter)) false true)
          ;[1 1 1] Fireworks
          (Utilities|FlowControl|DoN (Math|Conversions|ToInteger(Byte) (Utilities|String|Right (Variables|/Game/MarioPlatformer/Blueprints/Framework/BP_PlayerController.BP_PlayerController_C|GetFormattedTime (Variables|Default|GetPlayerController)) 1)) :!label _label
            (:Exit
              (Utilities|FlowControl|Delay 0.5)
              (bind _output_get_4 (Variables|Default|SetFireworksLocation (Math|Random|RandomPointinBoundingBox (Transformation|GetWorldLocation _fireworks_area) (Variables|/Script/Engine.BoxComponent|GetBoxExtent _fireworks_area))))
              (Audio|PlaySoundatLocation "/Game/StarterContent/Audio/Explosion_Cue.Explosion_Cue" _output_get_4 "0, 0, 0" 1.0 1.0 0.0 0 0 0 0)
              (Niagara|SpawnSystematLocation "/Game/Stylized_VFX_StPack/Particles/P_ExplosionEnergy_03.P_ExplosionEnergy_03" _output_get_4 "0, 0, 0" "5.000000,5.000000,5.000000")
              (Game|SpawnActorfromClass "/Game/MarioPlatformer/Blueprints/BP_Points.BP_Points_C" (Math|Transform|MakeTransform _output_get_4) "Undefined" "MultiplyWithRoot" 0 _fireworkspoints 0)
              (Default|AddPoints (Variables|Default|GetPlayerController) _fireworkspoints)
              (goto _label))))))))

(event EventBeginPlay)

(fn ConstructionScript)