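; BP_Pickup_Coin is a collectible coin pickup for a Mario-style platformer.
; On BeginPlay it caches the BP_PlayerController.
; When the player character overlaps its sphere collision, it adds NumCoins through the controller, plays a 2D coin sound with a fade-out, spawns an explosion particle at its location and destroys itself.
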(event OnComponentBeginOverlap(SphereCollision)
  (params (OverlappedComponent :type Primitive%20Component%20Object%20Reference) (OtherActor :type Actor%20Object%20Reference) (OtherComp :type Primitive%20Component%20Object%20Reference) (OtherBodyIndex :type Integer) (bFromSweep :type Boolean) (SweepResult :type Hit%20Result%20Structure%20%28by%20ref%29))
  ;[1 1 1] Picked Up
  (if (== OtherActor (Game|GetPlayerCharacter 0))
    (Default|AddCoins (Variables|Default|GetPlayerController) (Variables|Default|GetNumCoins))
    (bind _returnvalue (Audio|SpawnSound2D "/Game/MarioPlatformer/Audio/Mario_Coin_Modified.Mario_Coin_Modified" 1.0 1.0 0.0 0))
    (Audio|Components|Audio|FadeOut _returnvalue 0.6 0.0 "Linear" :!class /Script/Engine.AudioComponent)
    (Effects|SpawnEmitteratLocation "/Game/StarterContent/Particles/P_Explosion.P_Explosion" (Transformation|GetActorLocation))
    (Actor|DestroyActor)))

(event EventBeginPlay
  (bind _asbp_player_controller (Utilities|Casting|CastToBP_PlayerController (Game|GetPlayerController 0)))
  (Variables|Default|SetPlayerController _asbp_player_controller))

(fn ConstructionScript)