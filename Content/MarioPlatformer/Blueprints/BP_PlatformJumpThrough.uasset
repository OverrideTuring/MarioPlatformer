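; BP_PlatformJumpThrough is a one-way platform the player can jump up through and drop down from.
; Entering the bottom trigger with a near-vertical (+Z) impact normal disables Platform collision, and leaving that trigger restores it.
; The top trigger tracks whether the player stands on the platform, letting IA_JumpDown disable collision only then.
; All overlap checks respond only to player character 0.
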(event OnComponentBeginOverlap(BottomCollision)
  (params (OverlappedComponent :type Primitive%20Component%20Object%20Reference) (OtherActor :type Actor%20Object%20Reference) (OtherComp :type Primitive%20Component%20Object%20Reference) (OtherBodyIndex :type Integer) (bFromSweep :type Boolean) (SweepResult :type Hit%20Result%20Structure%20%28by%20ref%29))
  ;[1 1 1] Set Jump Through Collision
  (if (and (== OtherActor (Game|GetPlayerCharacter 0)) (Utilities|Operators|EqualEqual (.ImpactNormal (Collision|BreakHitResult SweepResult)) "0.000000,0.000000,1.000000" 0.1))
    (Collision|SetCollisionEnabled (Variables|Default|GetPlatform) "NoCollision")))

(event OnComponentEndOverlap(BottomCollision)
  (params (OverlappedComponent :type Primitive%20Component%20Object%20Reference) (OtherActor :type Actor%20Object%20Reference) (OtherComp :type Primitive%20Component%20Object%20Reference) (OtherBodyIndex :type Integer))
  ;[1 1 1] Set Jump Through Collision
  (if (== (Game|GetPlayerCharacter 0) OtherActor)
    (Collision|SetCollisionEnabled (Variables|Default|GetPlatform) "QueryAndPhysics")))

(event OnComponentBeginOverlap(TopCollision)
  (params (OverlappedComponent :type Primitive%20Component%20Object%20Reference) (OtherActor :type Actor%20Object%20Reference) (OtherComp :type Primitive%20Component%20Object%20Reference) (OtherBodyIndex :type Integer) (bFromSweep :type Boolean) (SweepResult :type Hit%20Result%20Structure%20%28by%20ref%29))
  ;[1 1 1] Judge whether on Platform
  (if (== OtherActor (Game|GetPlayerCharacter 0))
    (Variables|Default|SetOnPlatform true)))

(event OnComponentEndOverlap(TopCollision)
  (params (OverlappedComponent :type Primitive%20Component%20Object%20Reference) (OtherActor :type Actor%20Object%20Reference) (OtherComp :type Primitive%20Component%20Object%20Reference) (OtherBodyIndex :type Integer))
  ;[1 1 1] Judge whether on Platform
  (if (== (Game|GetPlayerCharacter 0) OtherActor)
    (Variables|Default|SetOnPlatform false)))

(event Input|EnhancedActionEvents|EnhancedInputActionIA_JumpDown
  (params (ActionValue :type Boolean) (ElapsedSeconds :type Float%20%28double-precision%29) (TriggeredSeconds :type Float%20%28double-precision%29) (InputAction :type Input%20Action%20Object%20Reference :default "/Game/ThirdPerson/Input/Actions/IA_JumpDown.IA_JumpDown"))
  ;[1 1 1] Jump Down
  (if (Variables|Default|GetOnPlatform)
    (Collision|SetCollisionEnabled (Variables|Default|GetPlatform) "NoCollision")))

(fn ConstructionScript)