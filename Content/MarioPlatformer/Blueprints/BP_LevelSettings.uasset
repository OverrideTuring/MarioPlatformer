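; Level settings actor for the Mario-style platformer that runs the countdown timer, music and level completion.
; A looping timer updates the player controller, kills the player at zero, and at the warning time plays a jingle before resuming music slightly pitched up.
; Player death stops music and timer; respawn reruns setup.
; The end flag's completion event converts remaining seconds into points through a delayed loop, then calls the game mode's LevelOver with the next level.
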(event Custom|Player%20Respawned_Event
  (bind _timelimit (Variables|Default|GetTimeLimit))
  (Audio|Components|Audio|SetPitchMultiplier (Variables|Default|GetLevelMusic) 1.0)
  (Utilities|FlowControl|Sequence
    (:then_0
      ;[1 1 1] Bind Player Respawned Event
      (Utilities|FlowControl|DoOnce false
        (:Completed
          (bind _asbp_third_person_game_mode (Utilities|Casting|CastToBP_ThirdPersonGameMode (Game|GetGameMode)))
          (EventDispatchers|AssignPlayerRespawned _asbp_third_person_game_mode (delegate Custom|Player%20Respawned_Event)))))
    (:then_1
      ;[1 1 1] Bind Player Death Event
      (bind _asbp_third_person_character (Utilities|Casting|CastToBP_ThirdPersonCharacter (Game|GetPlayerCharacter 0)))
      (EventDispatchers|AssignPlayerDeathSequence _asbp_third_person_character (delegate Custom|Player%20Death%20Sequence_Event)))
    (:then_2
      ;[1 1 1] Set Level Time
      (bind _asbp_player_controller (Utilities|Casting|CastToBP_PlayerController (Game|GetPlayerController 0)))
      (bind _output_get (Variables|Default|SetPlayerController _asbp_player_controller))
      (Default|UpdateTime _output_get _timelimit)
      (Variables|Default|SetCurrentTime _timelimit))
    (:then_3
      ;[1 1 1] Play Level Music
      (Audio|Components|Audio|SetSound (Variables|Default|GetLevelMusic) (Variables|Default|GetCurrentLevelMusic))
      (Utilities|FlowControl|Delay 0.75)
      (Audio|Components|Audio|Play (Variables|Default|GetLevelMusic) 0.0))
    (:then_4
      ;[1 1 1] Set Timer and Change Music
      (Utilities|FlowControl|RetriggerableDelay 1.0)
      (bind _returnvalue (Utilities|Time|SetTimerbyEvent (delegate Custom|Update%20Time) 1.0 true))
      (Variables|Default|SetLevelTimer _returnvalue))
    (:then_5
      ;[1 1 1] Level Complete
      (EventDispatchers|AssignLevelComplete (Variables|Default|GetEndLevelFlag) (delegate Custom|Level%20Complete_Event)))))

(event Custom|Update%20Time
  (bind _timerunningoutwarningmusic (Variables|Default|GetTimeRunningOutWarningMusic))
  (bind _levelmusic (Variables|Default|GetLevelMusic))
  ;[1 1 1] Set Timer and Change Music
  (bind _result (Math|Integer|DecrementInt (Variables|Default|GetCurrentTime))
    (:%20%20
      (Default|UpdateTime (Variables|Default|GetPlayerController) _result)
      (if (<= _result 0)
        (bind _asbp_third_person_character (Utilities|Casting|CastToBP_ThirdPersonCharacter (Game|GetPlayerCharacter 0)))
        (Default|PlayerDies _asbp_third_person_character)
        (elif (== _result (Variables|Default|GetWarningTime))
          (Class|AudioComponent|SetPaused _levelmusic true)
          (Audio|Components|Audio|Play _timerunningoutwarningmusic 0.0)
          (bind _assound_wave (Utilities|Casting|CastToSoundWave (Variables|/Script/Engine.AudioComponent|GetSound _timerunningoutwarningmusic)))
          (Utilities|FlowControl|Delay (+ (Variables|/Script/Engine.SoundBase|GetDuration _assound_wave) 0.5))
          (Audio|Components|Audio|SetPitchMultiplier _levelmusic 1.05)
          (Class|AudioComponent|SetPaused _levelmusic false))))))

(event Custom|Player%20Death%20Sequence_Event
  ;[1 1 1] Bind Player Death Event
  (Audio|Components|Audio|Stop (Variables|Default|GetTimeRunningOutWarningMusic))
  (Utilities|Time|ClearandInvalidateTimerbyHandle (Variables|Default|GetLevelTimer)))

(event Custom|Level%20Complete_Event
  (bind _playercontroller (Variables|Default|GetPlayerController))
  ;[1 1 1] Level Complete
  (Utilities|Time|PauseTimerbyHandle (Variables|Default|GetLevelTimer))
  (Audio|Components|Audio|Stop (Variables|Default|GetLevelMusic))
  (Utilities|FlowControl|Delay 3.0)
  (Components|Activation|Activate (Variables|Default|GetLevelCompleteMusic) false)
  (if (> (Variables|Default|GetCurrentTime) 0) :!label _label
    (Utilities|FlowControl|Delay 0.05)
    (bind _result (Math|Integer|DecrementInt (Variables|Default|GetCurrentTime))
      (:%20%20
        (Default|UpdateTime _playercontroller _result)
        (Default|AddPoints _playercontroller (Variables|Default|GetPointsPerSec))
        (Audio|PlaySound2D "/Engine/VREditor/Sounds/UI/Camera_Shutter.Camera_Shutter" 1.0 1.0 0.0 0 0)
        (goto _label)))
    (else
      (Utilities|FlowControl|Delay 1.0)
      (Default|LevelOver (.AsBP%20Third%20Person%20Game%20Mode (Utilities|Casting|CastToBP_ThirdPersonGameMode (Game|GetGameMode))) (Variables|Default|GetNextLevel)))))

(event EventBeginPlay
  (bind _timelimit (Variables|Default|GetTimeLimit))
  (Utilities|FlowControl|Sequence
    (:then_0
      ;[1 1 1] Bind Player Respawned Event
      (Utilities|FlowControl|DoOnce false
        (:Completed
          (bind _asbp_third_person_game_mode (Utilities|Casting|CastToBP_ThirdPersonGameMode (Game|GetGameMode)))
          (EventDispatchers|AssignPlayerRespawned _asbp_third_person_game_mode (delegate Custom|Player%20Respawned_Event)))))
    (:then_1
      ;[1 1 1] Bind Player Death Event
      (bind _asbp_third_person_character (Utilities|Casting|CastToBP_ThirdPersonCharacter (Game|GetPlayerCharacter 0)))
      (EventDispatchers|AssignPlayerDeathSequence _asbp_third_person_character (delegate Custom|Player%20Death%20Sequence_Event)))
    (:then_2
      ;[1 1 1] Set Level Time
      (bind _asbp_player_controller (Utilities|Casting|CastToBP_PlayerController (Game|GetPlayerController 0)))
      (bind _output_get (Variables|Default|SetPlayerController _asbp_player_controller))
      (Default|UpdateTime _output_get _timelimit)
      (Variables|Default|SetCurrentTime _timelimit))
    (:then_3
      ;[1 1 1] Play Level Music
      (Audio|Components|Audio|SetSound (Variables|Default|GetLevelMusic) (Variables|Default|GetCurrentLevelMusic))
      (Utilities|FlowControl|Delay 0.75)
      (Audio|Components|Audio|Play (Variables|Default|GetLevelMusic) 0.0))
    (:then_4
      ;[1 1 1] Set Timer and Change Music
      (Utilities|FlowControl|RetriggerableDelay 1.0)
      (bind _returnvalue (Utilities|Time|SetTimerbyEvent (delegate Custom|Update%20Time) 1.0 true))
      (Variables|Default|SetLevelTimer _returnvalue))
    (:then_5
      ;[1 1 1] Level Complete
      (EventDispatchers|AssignLevelComplete (Variables|Default|GetEndLevelFlag) (delegate Custom|Level%20Complete_Event)))))

(fn ConstructionScript)