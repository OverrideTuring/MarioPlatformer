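; BP_Bullet is a bouncing projectile for the platformer that tells the player character when it is destroyed.
; On each projectile bounce, hitting a wall-like surface makes it explode at once, while mostly horizontal surfaces let it bounce until a small bounce limit is reached.
; Exploding spawns an effect with an attached sound and destroys the actor, whose OnDestroyed event calls BulletDestroy on the cached BP_ThirdPersonCharacter.
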(event OnProjectileBounce(ProjectileMovement)
  (params (ImpactResult :type Hit%20Result%20Structure%20%28by%20ref%29) (ImpactVelocity :type Vector%20%28by%20ref%29 :default "0, 0, 0"))
  (bind _sphere (Variables|Default|GetSphere))
  (bind _returnvalue (Transformation|GetWorldTransform _sphere))
  (if (< (.z (Math|Vector|VectorGetAbs (.Normal (Collision|BreakHitResult ImpactResult)))) 0.9)
    (bind _returnvalue_2 (Niagara|SpawnSystematLocation "/Game/Stylized_VFX_StPack/VR/VR_Particles/P_VR_ExplosionEnergy_03.P_VR_ExplosionEnergy_03" (.location _returnvalue) (.rotation _returnvalue) (.scale _returnvalue) :!label _label))
    (Audio|SpawnSoundAttached "/Game/StarterContent/Audio/Explosion_Cue.Explosion_Cue" _returnvalue_2 "None" "0, 0, 0" "0, 0, 0" "KeepRelativeOffset" false 1.0 1.0 0.0 0 0)
    (Actor|DestroyActor)
    (else
      (bind _result (Math|Integer|IncrementInt (Variables|Default|GetBounceCount))
        (:%20%20
          (if (>= _result 2)
            (goto _label)))))))

(event Custom|OnDestroyed_Event
  (params (DestroyedActor :type Actor%20Object%20Reference))
  (Default|BulletDestroy (Variables|Default|GetPlayerCharacter)))

(event EventBeginPlay
  (EventDispatchers|BindEventtoOnDestroyed (delegate Custom|OnDestroyed_Event))
  (bind _asbp_third_person_character (Utilities|Casting|CastToBP_ThirdPersonCharacter (Game|GetPlayerCharacter 0)))
  (Variables|Default|SetPlayerCharacter _asbp_third_person_character))

(fn ConstructionScript)