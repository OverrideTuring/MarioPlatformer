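; Player controller for a Mario-style platformer that owns the HUD and pause menu and tracks coins, points, lives and level time.
; The pause input toggles the menu, game pause and sound, using cursor visibility as the state flag.
; Events update the stats, converting each hundred coins into lives and formatting time as minutes and seconds.
; Running out of lives plays a sound, then calls GameOver on the cached game mode after a delay.
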(event Custom|Add%20Coins
  (params (NumCoins :type Integer))
  ;[1 1 1] Add Coins
  (if (>= (+ NumCoins (Variables|Default|GetCoinCount)) 100)
    (Variables|Default|SetCoinCount (Math|Integer|%(Integer) (+ NumCoins (Variables|Default|GetCoinCount)) 100))
    (CallFunction|AdjustLives (/ (+ NumCoins (Variables|Default|GetCoinCount)) 100))
    (Audio|PlaySound2D "/Game/MarioPlatformer/Audio/Mario_1up.Mario_1up" 1.0 1.0 0.0 0 0)
    (else
      (Variables|Default|SetCoinCount (+ NumCoins (Variables|Default|GetCoinCount))))))

(event Custom|Update%20Time
  (params (Updated%20Time :type Integer))
  ;[1 1 1] Update Time
  (bind _output_get (Variables|Default|SetLevelTime Updated%20Time))
  (Variables|Default|SetFormattedTime (CallFunction|ConvertSecondstoMMSS _output_get)))

(event Custom|Adjust%20Lives
  (params (DeltaLives :type Integer))
  ;[1 1 1] Adjust Lives
  (bind _output_get (Variables|Default|SetLives (Math|Integer|Clamp(Integer) (+ DeltaLives (Variables|Default|GetLives)) 0 999)))
  (if (== _output_get 0)
    (Audio|PlaySound2D "/Game/MarioPlatformer/Audio/Mario_GameOver.Mario_GameOver" 1.0 1.0 0.0 0 0)
    (Utilities|FlowControl|Delay 4.0)
    (Default|GameOver (Variables|Default|GetGameMode) false)))

(event Custom|Add%20Points
  (params (AddedPoints :type Integer))
  ;[1 1 1] Add Points
  (Variables|Default|SetPoints (+ AddedPoints (Variables|Default|GetPoints))))

(event Input|EnhancedActionEvents|EnhancedInputActionIA_Pause
  (params (ActionValue :type Boolean) (ElapsedSeconds :type Float%20%28double-precision%29) (TriggeredSeconds :type Float%20%28double-precision%29) (InputAction :type Input%20Action%20Object%20Reference :default "/Game/ThirdPerson/Input/Actions/IA_Pause.IA_Pause"))
  (bind _pausemenu (Variables|Default|GetPauseMenu))
  (:Started
    (if (Variables|Default|GetbShowMouseCursor)
      (Widget|RemovefromParent _pausemenu)
      (Variables|Default|SetbShowMouseCursor false)
      (Audio|PlaySound2D "/Engine/VREditor/Sounds/UI/Floating_UI_Close.Floating_UI_Close" 1.0 1.0 0.0 0 0)
      (Game|SetGamePaused false)
      (else
        (UserInterface|Viewport|AddtoViewport _pausemenu 0)
        (Variables|Default|SetbShowMouseCursor true)
        (Audio|PlaySound2D "/Game/MarioPlatformer/Audio/Mario_Pause.Mario_Pause" 1.0 1.0 0.0 0 0)
        (Game|SetGamePaused true)
        (Input|SetInputModeGameandUI self (Variables|Default|GetPauseMenu) "DoNotLock" true true)))))

(event EventBeginPlay
  ;[1 1 1] Create Widget
  (bind _returnvalue (UserInterface|CreateWidget "/Game/MarioPlatformer/UI/WBP_HUD.WBP_HUD_C"))
  (UserInterface|Viewport|AddtoViewport _returnvalue 0)
  ;[1 1 1] Reference to Game Mode
  (bind _asbp_third_person_game_mode (Utilities|Casting|CastToBP_ThirdPersonGameMode (Game|GetGameMode)))
  (Variables|Default|SetGameMode _asbp_third_person_game_mode)
  ;[1 1 1] Create Pause Menu
  (bind _returnvalue_2 (UserInterface|CreateWidget "/Game/MarioPlatformer/UI/WBP_PauseMenu.WBP_PauseMenu_C"))
  (Variables|Default|SetPauseMenu _returnvalue_2))

(fn ConstructionScript)

(fn ConvertSecondstoMMSS
  (params (Seconds :type Integer))
  (return (Utilities|String|Append (Utilities|String|ToString(Text) (Utilities|Text|ToText(Integer) (/ Seconds 60) false true 2)) ":" (Utilities|String|ToString(Text) (Utilities|Text|ToText(Integer) (Math|Integer|%(Integer) Seconds 60) false true 2)))))