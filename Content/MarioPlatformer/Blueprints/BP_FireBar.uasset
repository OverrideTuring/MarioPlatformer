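; BP_FireBar is a Mario-style rotating fire bar hazard that launches and adjusts the hit points of the player on contact.
; The construction script stacks flame balls along local Z as mesh instances, fits the collision box to their count, spacing and size, and sets the RotatingMovement rate.
; On overlap, it overrides the character's velocity and calls AdjustHitPoints, with a DoOnce and Delay enforcing a cooldown between hits.
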(event OnComponentBeginOverlap(BoxCollision)
  (params (OverlappedComponent :type Primitive%20Component%20Object%20Reference) (OtherActor :type Actor%20Object%20Reference) (OtherComp :type Primitive%20Component%20Object%20Reference) (OtherBodyIndex :type Integer) (bFromSweep :type Boolean) (SweepResult :type Hit%20Result%20Structure%20%28by%20ref%29))
  ;[1 1 1] Hit Player
  (bind _asbp_third_person_character (Utilities|Casting|CastToBP_ThirdPersonCharacter OtherActor))
  (Utilities|FlowControl|DoOnce false :!label _label
    (:Completed
      (Variables|/Script/Engine.MovementComponent|SetVelocity (Variables|/Script/Engine.Character|GetCharacterMovement _asbp_third_person_character) (Variables|Default|GetPlayerHitVelocity))
      (Default|AdjustHitPoints _asbp_third_person_character (Variables|Default|GetHitPointsModifier))
      (Utilities|FlowControl|Delay (Variables|Default|GetCoolDown))
      (goto _label Reset))))

(fn ConstructionScript
  (bind _flameballnum (Variables|BarCustomization|GetFlameBallNum))
  (bind _flameballdistanceapart (Variables|BarCustomization|GetFlameBallDistanceApart))
  (bind _boxcollision (Variables|Default|GetBoxCollision))
  (bind _flameballsize (Variables|BarCustomization|GetFlameBallSize))
  (bind _returnvalue (- _flameballnum 1))
  (bind _returnvalue_2 (* _flameballsize "50.000000,50.000000,50.000000"))
  (bind _returnvalue_3 (* _flameballdistanceapart _returnvalue))
  (bind _returnvalue_4 (/ _returnvalue_3 2))
  (bind _returnvalue_5 (Math|Conversions|ToFloat(Integer) _returnvalue_4))
  (for _index (range 0 _returnvalue)
    ;[1 1 1] Create Flame Balls
    (Components|InstancedStaticMesh|AddInstance (Variables|Default|GetInstancedStaticMesh) (Math|Transform|MakeTransform (Math|Vector|MakeVector 0.0 0.0 (Math|Conversions|ToFloat(Integer) (* _index _flameballdistanceapart))) "0, 0, 0" (Variables|BarCustomization|GetFlameBallSize)) false))
  (Utilities|FlowControl|Sequence
    (:then_0
      ;[1 1 1] Set Collision Box
      (Transformation|SetRelativeLocation _boxcollision (Math|Vector|MakeVector 0.0 0.0 _returnvalue_5) false false)
      (Components|Box|SetBoxExtent _boxcollision (Math|Vector|MakeVector (.x _returnvalue_2) (.y _returnvalue_2) (+ _returnvalue_5 (.z _returnvalue_2))) true))
    (:then_1
      ;[1 1 1] Set Rotation Rate
      (Variables|/Script/Engine.RotatingMovementComponent|SetRotationRate (Variables|Default|GetRotatingMovement) (Variables|BarCustomization|GetRotationRate)))))