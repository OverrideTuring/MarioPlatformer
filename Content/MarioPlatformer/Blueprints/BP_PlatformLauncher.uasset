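; Mushroom bounce platform that launches the player character when it lands on the hat.
; Overlapping BottomCollision disables hat collision for the player to pass through, restoring it when the overlap ends.
; A vertical hit on the hat launches the player, spawns dirt particles and plays a scale timeline, gated by a DoOnce with delayed reset.
; The construction script sizes the hat and stacks instanced trunk segments from the endpoint's height, upward or downward.
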(event OnComponentBeginOverlap(BottomCollision)
  (params (OverlappedComponent :type Primitive%20Component%20Object%20Reference) (OtherActor :type Actor%20Object%20Reference) (OtherComp :type Primitive%20Component%20Object%20Reference) (OtherBodyIndex :type Integer) (bFromSweep :type Boolean) (SweepResult :type Hit%20Result%20Structure%20%28by%20ref%29))
  (if (== OtherActor (Game|GetPlayerCharacter 0))
    (Collision|SetCollisionEnabled (Variables|Default|GetMushroomHat) "NoCollision")))

(event OnComponentEndOverlap(BottomCollision)
  (params (OverlappedComponent :type Primitive%20Component%20Object%20Reference) (OtherActor :type Actor%20Object%20Reference) (OtherComp :type Primitive%20Component%20Object%20Reference) (OtherBodyIndex :type Integer))
  (if (== (Game|GetPlayerCharacter 0) OtherActor)
    (Collision|SetCollisionEnabled (Variables|Default|GetMushroomHat) "QueryAndPhysics")))

(event OnComponentHit(MushroomHat)
  (params (HitComponent :type Primitive%20Component%20Object%20Reference) (OtherActor :type Actor%20Object%20Reference) (OtherComp :type Primitive%20Component%20Object%20Reference) (NormalImpulse :type Vector :default "0, 0, 0") (Hit :type Hit%20Result%20Structure%20%28by%20ref%29))
  (bind _returnvalue (Game|GetPlayerCharacter 0))
  (bind (_bblockinghit _binitialoverlap _time _distance _location _impactpoint _normal _impactnormal) (Collision|BreakHitResult Hit))
  (if (== OtherActor _returnvalue)
    (if (Class|KismetMathLibrary|EqualExactlyVectorVector _impactnormal "0.000000,0.000000,-1.000000")
      (Utilities|FlowControl|DoOnce false :!label _label
        (:Completed
          (Character|LaunchCharacter _returnvalue (Variables|Default|GetLaunchVelocity) false false)
          (Niagara|SpawnSystematLocation "/Game/A_Surface_Footstep/Niagara_FX/ParticleSystems/PSN_Dirt_Surface.PSN_Dirt_Surface" _impactpoint "0, 0, 0" "3.000000,3.000000,3.000000")
          (bind _scale (Timeline|Scale%20Timeline PlayFromStart)
            (:Update
              (Transformation|SetWorldScale3D (Variables|Default|GetMushroomHat) (* _scale (Variables|Default|GetMushroomHatScale)))
              (Utilities|FlowControl|Delay 0.2)
              (goto _label Reset))))))))

(fn ConstructionScript
  (bind _mushroomtrunkendpoint (Variables|Default|GetMushroomTrunkEndPoint))
  (bind _returnvalue (/ (.z _mushroomtrunkendpoint) 1e+02))
  (bind _returnvalue_2 (Math|Float|Truncate _returnvalue))
  (Transformation|SetWorldScale3D (Variables|Default|GetMushroomHat) (Variables|Default|GetMushroomHatScale))
  (if (> _returnvalue_2 0)
    (for _index (range 1 _returnvalue_2)
      (Components|InstancedStaticMesh|AddInstance (Variables|Default|GetMushroomTrunk) (Math|Transform|MakeTransform (Math|Vector|MakeVector 0.0 0.0 (* _index 100)) "0, 0, 0" "1.000000,1.000000,1.000000") false))
    (else
      (for _index_2 (range _returnvalue_2 0)
        (Components|InstancedStaticMesh|AddInstance (Variables|Default|GetMushroomTrunk) (Math|Transform|MakeTransform (Math|Vector|MakeVector 0.0 0.0 (* _index_2 100)) "0, 0, 0" "1.000000,1.000000,1.000000") false)))))