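; BP_PlatformJumpThrough_Movable is a moving variant of a jump-through platform for a Mario-style platformer.
; On BeginPlay it sets the timeline's play rate from MoveRate and starts it.
; Each timeline update lerps the Platform component's relative location between StartPosition and EndPosition, without sweeping.
; Its construction script only calls the parent's, leaving setup to the parent class.
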(event EventBeginPlay
  (Components|Timeline|SetPlayRate (Variables|Default|GetPosition%20Timeline) (Variables|Default|GetMoveRate))
  (bind _alpha (Timeline|Position%20Timeline Play)
    (:Update
      (Transformation|SetRelativeLocation (Variables|Default|GetPlatform) (Math|Vector|Lerp(Vector) (Variables|Default|GetStartPosition) (Variables|Default|GetEndPosition) _alpha) false false))))

(fn ConstructionScript
  (|CallParentFunction))