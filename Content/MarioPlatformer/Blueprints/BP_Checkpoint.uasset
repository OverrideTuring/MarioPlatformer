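; BP_Checkpoint is a platformer checkpoint that updates the player's respawn location when the third-person character first overlaps its box.
; A DoOnce gate writes the RespawnPoint component's world transform into the game mode's SpawnTransform and plays a sound.
; A timeline then rotates the flag arm, and on finish plays a second sound, spawns a level-up effect near the flag and swaps the flag to a green material.
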(event OnComponentBeginOverlap(BoxCollision)
  (params (OverlappedComponent :type Primitive%20Component%20Object%20Reference) (OtherActor :type Actor%20Object%20Reference) (OtherComp :type Primitive%20Component%20Object%20Reference) (OtherBodyIndex :type Integer) (bFromSweep :type Boolean) (SweepResult :type Hit%20Result%20Structure%20%28by%20ref%29))
  (bind _flag (Variables|Default|GetFlag))
  (bind _returnvalue (Transformation|GetWorldTransform _flag))
  (Utilities|Casting|CastToBP_ThirdPersonCharacter OtherActor)
  (Utilities|FlowControl|DoOnce false
    (:Completed
      (bind _asbp_third_person_game_mode (Utilities|Casting|CastToBP_ThirdPersonGameMode (Game|GetGameMode)))
      (Variables|/Game/ThirdPerson/Blueprints/BP_ThirdPersonGameMode.BP_ThirdPersonGameMode_C|SetSpawnTransform _asbp_third_person_game_mode (Transformation|GetWorldTransform (Variables|Default|GetRespawnPoint)))
      (Audio|PlaySound2D "/Engine/VREditor/Sounds/UI/Enter_Simulate.Enter_Simulate" 1.0 1.0 0.0 0 0)
      (bind _rotation_alpha (Timeline|Rotation%20Timeline PlayFromStart)
        (:Update
          (Transformation|SetRelativeRotation (Variables|Default|GetFlagArm) (Math|Rotator|Lerp(Rotator) (Variables|/Script/Engine.SceneComponent|GetRelativeRotation (Variables|Default|GetFlagArm)) "0, 0, 0" _rotation_alpha) false false))
        (:Finished
          (Audio|PlaySound2D "/Engine/EditorSounds/GamePreview/EndSimulate_Cue.EndSimulate_Cue" 1.0 1.0 0.0 0 0)
          (Niagara|SpawnSystematLocation "/Game/Stylized_VFX_StPack/Particles/P_LvlUp.P_LvlUp" (- (.location _returnvalue) "0.000000,0.000000,100.000000") (.rotation _returnvalue) (* (.scale _returnvalue) "10.000000,10.000000,10.000000"))
          (Rendering|Material|SetMaterial (Variables|Default|GetFlag) 0 "/Engine/EngineDebugMaterials/VertexColorViewMode_GreenOnly.VertexColorViewMode_GreenOnly"))))))

(fn ConstructionScript)