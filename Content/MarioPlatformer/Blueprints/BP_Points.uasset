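; BP_Points is a short-lived actor in the Mario platformer that displays an animated points value through its Widget component.
; On BeginPlay it casts the component's widget to WBP_Points, writes its Points value into the text and plays the points animation.
; It waits for the animation's end time, then destroys itself, so it only displays the value and does not change any score.
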(event EventBeginPlay
  (bind _aswbp_points (Utilities|Casting|CastToWBP_Points (UserInterface|GetWidget (Variables|Default|GetWidget))))
  (Rendering|Components|TextRender|SetText (Variables|/Game/MarioPlatformer/UI/WBP_Points.WBP_Points_C|GetTextPoints _aswbp_points) (Utilities|Text|ToText(Integer) (Variables|Default|GetPoints)))
  (UserInterface|Animation|PlayAnimation _aswbp_points (Variables|/Game/MarioPlatformer/UI/WBP_Points.WBP_Points_C|GetPointsAnimation _aswbp_points) 0.0 1 "Forward" 1.0 false)
  (Utilities|FlowControl|Delay (Class|WidgetAnimation|GetEndTime (Variables|/Game/MarioPlatformer/UI/WBP_Points.WBP_Points_C|GetPointsAnimation _aswbp_points)))
  (Actor|DestroyActor))

(fn ConstructionScript)